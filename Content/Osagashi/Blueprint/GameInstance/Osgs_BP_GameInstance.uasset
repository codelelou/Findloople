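; Game instance for Osagashi that owns the FlagMaster object and handles game restart, failure and salvage.
; SetupFlagMaster creates, sets up and starts FlagMaster only if it is not yet valid; it runs on Init and lazily through GetFlagMaster.
; RestartGame, FailedGame and SalvageGame respectively restart the flags, force a failure or update histories, then all reopen the top level.
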(event Custom|SetupFlagMaster
  ;[1 1 1] FlagMaster
  (Utilities|IsValid (stale _output_get)
    (:Is%20Not%20Valid
      (bind _returnvalue (Game|ConstructObjectfromClass (Variables|Default|GetFlagMasterClass)))
      (bind _output_get (Variables|Default|SetFlagMaster _returnvalue))
      (Utilities|FlowControl|Sequence
        (:then_0
          (Default|SetupFlags _output_get))
        (:then_1
          (Default|Start _output_get))))))

(event EventFailedGame
  (Utilities|FlowControl|Sequence
    (:then_0
      (bind _returnvalue (CallFunction|GetFlagMaster))
      (Default|ForceFailed _returnvalue false))
    (:then_1
      (Game|OpenLevel(byObjectReference) (Variables|Default|GetTopLevel)))))

(event EventSalvageGame
  (Utilities|FlowControl|Sequence
    (:then_0
      (bind _returnvalue (CallFunction|GetFlagMaster))
      (Default|UpdateHistories _returnvalue))
    (:then_1
      (Game|OpenLevel(byObjectReference) (Variables|Default|GetTopLevel)))))

(event EventRestartGame
  (Utilities|FlowControl|Sequence
    (:then_0
      (bind _returnvalue (CallFunction|GetFlagMaster))
      (Default|Restart _returnvalue))
    (:then_1
      (Game|OpenLevel(byObjectReference) (Variables|Default|GetTopLevel)))))

(event EventInit
  (CallFunction|SetupFlagMaster))

(fn GetFlagMaster
  (CallFunction|SetupFlagMaster)
  (return (Variables|Default|GetFlagMaster)))