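; Base actor component for answering in the Osagashi game, posting a flag answer to the FlagMaster.
; FlagMaster entry and judged events toggle standby, driving a find-or-create widget's visibility and DoOnce-gated input hooks left empty here.
; Answer checks actors implementing the answer interface for one reporting a find; otherwise it deliberately posts the opposite of the current flag.
; Accepted posts trigger the widget's answer-finished message.
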(event Custom|HandleEntry
  (Utilities|FlowControl|DoOnce false
    (:Completed
      (bind _returnvalue (CallFunction|GetFlagMaster))
      (if (not (Default|IsNoPickCurrentRound _returnvalue))
        (CallFunction|SetStandby true)))))

(event Custom|SetupFlagMaster
  (bind _returnvalue (CallFunction|GetFlagMaster))
  (Utilities|FlowControl|Sequence
    (:then_0
      (EventDispatchers|AssignOnEntry _returnvalue (delegate Custom|HandleEntry)))
    (:then_1
      (EventDispatchers|AssignOnJudged _returnvalue (delegate Custom|HandleJudged)))))

(event Custom|SetAnswerResult
  (params (Answer :type Boolean) (Valid :type Boolean) (Success :type Boolean) (Ended :type Boolean))
  ;[1 1 1] Answer
  (if Valid
    (bind _returnvalue (CallFunction|GetUserWidget))
    (Class|OsgsBPIAnswerUserWidget|PlayAnswerFinished(Message) _returnvalue)))

(event Custom|HandleEnableInput
  ;[1 1 1] Input
)

(event Custom|HandleDisableInput
  ;[1 1 1] Input
)

(event Custom|UpdateInput
  (params (Standby :type Boolean))
  ;[1 1 1] Input
  (if Standby
    (Utilities|FlowControl|DoOnce false :!label _label
      (:Completed
        (Utilities|FlowControl|Sequence
          (:then_0
            (CallFunction|HandleEnableInput))
          (:then_1
            (goto _label_2 Reset)))))
    (else
      (Utilities|FlowControl|DoOnce true :!label _label_2
        (:Completed
          (Utilities|FlowControl|Sequence
            (:then_0
              (CallFunction|HandleDisableInput))
            (:then_1
              (goto _label Reset))))))))

(event Custom|FailedAnswer
  ;[1 1 1] Answer
  (bind _returnvalue (CallFunction|GetFlagMaster))
  (bind _returnvalue_2 (Default|IsCurrentFlag _returnvalue))
  (CallFunction|HandleAnswer (not _returnvalue_2)))

(event Custom|HandleJudged
  (params (Success :type Boolean))
  (Utilities|FlowControl|Sequence
    (:then_0
      (CallFunction|SetStandby false))
    (:then_1
      (Utilities|FlowControl|DoOnce false) ; enters at Reset
    )))

(event Custom|SetUserWidgetVisibility
  (params (Visibility :type Boolean))
  ;[1 1 1] Widget
  (bind _returnvalue (CallFunction|GetUserWidget))
  (Utilities|IsValid _returnvalue
    (:Is%20Valid
      (Widget|SetVisibility _returnvalue (select Visibility "SelfHitTestInvisible" "Collapsed")))))

(event Custom|SetStandby
  (params (Standby :type Boolean))
  (Utilities|FlowControl|Sequence
    (:then_0
      (CallFunction|SetUserWidgetVisibility Standby))
    (:then_1
      (CallFunction|UpdateInput Standby))))

(event Custom|Answer
  ;[1 1 1] Answer
  (if (stale Custom|SetStandby Standby)
    (bind _returnvalue (CallFunction|ValidAnswer))
    (if _returnvalue
      (CallFunction|HandleAnswer (Variables|Default|GetAnswerIsFlag))
      (else
        (CallFunction|FailedAnswer)))))

(event Custom|HandleAnswer
  (params (IsFlag :type Boolean))
  ;[1 1 1] Answer
  (bind _returnvalue (CallFunction|GetFlagMaster))
  (bind (_valid _success _ended) (Default|PostAnswer _returnvalue IsFlag))
  (CallFunction|SetAnswerResult IsFlag _valid _success _ended))

(event EventBeginPlay
  (if (Utilities|IsValidClass (Variables|Default|GetUserWidgetClass))
    (CallFunction|SetupFlagMaster)))

(event EventTick
  (params (DeltaSeconds :type Float%20%28single-precision%29)))

(fn GetUserWidget
  (bind _userwidgetclass (Variables|Default|GetUserWidgetClass))
  (bind _foundwidgets (Widget|GetAllWidgetsOfClass _userwidgetclass true))
  (Utilities|IsValid (Utilities|Array|Get(acopy) _foundwidgets)
    (:Is%20Valid
      (return (Utilities|Array|Get(acopy) _foundwidgets)))
    (:Is%20Not%20Valid
      (if (Utilities|IsValidClass _userwidgetclass)
        (bind _returnvalue (UserInterface|CreateWidget _userwidgetclass))
        (Utilities|FlowControl|Sequence
          (:then_0
            (UserInterface|Viewport|AddtoViewport _returnvalue 0))
          (:then_1
            (return _returnvalue)))))))

(fn ValidAnswer
  (bind _outactors (Actor|GetAllActorswithInterface "/Game/Osagashi/Blueprint/Actor/Answer/Osgs_BPI_Actor_Answer.Osgs_BPI_Actor_Answer_C")) ; 回答用アクターを検索
  (for _array_element _outactors
    (bind _returnvalue (Class|OsgsBPIActorAnswer|IsFindingAnswerActor(Message) _array_element))
    (if _returnvalue ; 回答用アクターを見つけている状態かどうか
      (return true)))
  (return false))