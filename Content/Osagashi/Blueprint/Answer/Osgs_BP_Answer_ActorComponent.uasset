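; Actor component that handles the player's Answer input in the Osagashi game.
; Enable and disable hooks from its parent toggle the owner's input and add or remove a high-priority Enhanced Input mapping context.
; The Answer action starts a hold message on the user widget using the hold time threshold, calls Answer when triggered, and stops the message on cancel or completion.
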(event Custom|UpdateInputSettings
  (params (Active :type Boolean))
  (bind _returnvalue (Game|GetPlayerController 0))
  (bind _mappingcontext (Variables|Default|GetMappingContext))
  (bind _returnvalue_2 (PlayerController|LocalPlayerSubsystems|GetEnhancedInputLocalPlayerSubsystem _returnvalue))
  (if Active
    (if (not (.ReturnValue (Class|EnhancedInputSubsystemInterface|HasMappingContext _returnvalue_2 _mappingcontext)))
      (Input|AddMappingContext _returnvalue_2 _mappingcontext 999 "(bIgnoreAllPressedKeysUntilRelease=True,bForceImmediately=False,bNotifyUserSettings=False)"))
    (else
      (Input|RemoveMappingContext _returnvalue_2 _mappingcontext "(bIgnoreAllPressedKeysUntilRelease=True,bForceImmediately=False,bNotifyUserSettings=False)"))))

(event Input|EnhancedActionEvents|EnhancedInputActionOsgs_IA_Answer
  (params (ActionValue :type Boolean) (ElapsedSeconds :type Float%20%28double-precision%29) (TriggeredSeconds :type Float%20%28double-precision%29) (InputAction :type Input%20Action%20Object%20Reference :default "/Game/Osagashi/Input/Osgs_IA_Answer.Osgs_IA_Answer"))
  (:Triggered
    (CallFunction|Answer))
  (:Started
    (bind _returnvalue (CallFunction|GetUserWidget))
    (Class|OsgsBPIAnswerUserWidget|StartAnswerHold(Message) _returnvalue (Variables|Default|GetHoldTimeThreshold)))
  (:Canceled
    (Class|OsgsBPIAnswerUserWidget|StopAnswerHold(Message) _returnvalue :!label _label))
  (:Completed
    (goto _label)))

(event EventBeginPlay
  (|CallParentFunction) ; このノードは無効になっているため呼び出せません。\n機能をビルドするにはピンをドラッグしてください。
)

(event EventTick
  (params (DeltaSeconds :type Float%20%28single-precision%29))
  (|CallParentFunction DeltaSeconds) ; このノードは無効になっているため呼び出せません。\n機能をビルドするにはピンをドラッグしてください。
)

(event EventHandleEnableInput
  (|CallParentFunction)
  (Utilities|FlowControl|Sequence
    (:then_0
      (CallFunction|UpdateInputSettings true))
    (:then_1
      (Input|EnableInput (Components|GetOwner) (Game|GetPlayerController 0)))))

(event EventHandleDisableInput
  (|CallParentFunction)
  (Utilities|FlowControl|Sequence
    (:then_0
      (CallFunction|UpdateInputSettings false))
    (:then_1
      (Input|DisableInput (Components|GetOwner) (Game|GetPlayerController 0)))))