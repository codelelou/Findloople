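; Level helper for the main stage of an anomaly-finding game, driving stage loading and answer checks from player-only trigger overlaps.
; Entry starts the FlagMaster and arms stage and answer triggers; front/back triggers alternately load the stage level instance at their transforms, using paired DoOnce gates.
; Answer triggers make FlagMaster post the answer or advance.
; Also handles fall salvage via GameInstance and optional start teleport to the unfound-anomaly guide.
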(event Custom|LoadStage
  (params (Level :type World%20Soft%20Object%20Reference) (Location :type Vector) (Rotation :type Rotator))
  ;[1 1 1] Load Stage
  (bind _returnvalue (Class|LevelStreamingDynamic|LoadLevelInstancebySoftObjectPtr Level Location Rotation "" 0 false))
  (Utilities|IsValid _returnvalue
    (:Is%20Valid
      (CallFunction|HandleLoadedStage _returnvalue))))

(event Custom|Entry
  ;[1 1 1] Entry
  (Utilities|FlowControl|DoOnce false
    (:Completed
      (Utilities|FlowControl|Sequence
        (:then_0
          (bind _returnvalue (CallFunction|GetFlagMaster))
          (Default|Entry _returnvalue))
        (:then_1
          (CallFunction|SetupAnswerTriggers)
          (CallFunction|SetupStageTriggers))))))

(event Custom|SetupEntryTriggers
  ;[1 1 1] Triggers
  ;;[1 1 1] Setup Triggers
  (CallFunction|BindTriggersBeginOverlap (Variables|Default|GetEntryTriggers)))

(event Custom|SetupTriggers
  ;[1 1 1] Triggers
  ;;[1 1 1] Setup Triggers
  (CallFunction|SetupEntryTriggers)
  (CallFunction|SetupSalvageTriggers))

(event Custom|Salvage
  ;[1 1 1] Salvage（想定外のルートで落下した場合のサルベージ処理）
  (Utilities|FlowControl|DoOnce false
    (:Completed
      (Class|OsgsBPIGameInstance|SalvageGame(Message) (Game|GetGameInstance)))))

(event Custom|HandleTeleportPlayerToUncheckedAnomalyGuide
  (bind _notfoundsguideplayertransform (Variables|Default|GetNotFoundsGuidePlayerTransform))
  (bind _returnvalue (Transformation|GetActorTransform _notfoundsguideplayertransform))
  ;[1 1 1] 見つけていないFlagの案内前にテレポート
  (Utilities|FlowControl|Sequence
    (:then_0
      (Transformation|Teleport (Game|GetPlayerCharacter 0) (.location _returnvalue) "0, 0, 0"))
    (:then_1
      (Pawn|SetControlRotation (Game|GetPlayerController 0) (.rotation _returnvalue)))))

(event Custom|SetupAnswerTriggers
  ;[1 1 1] Triggers
  ;;[1 1 1] Setup Triggers
  (CallFunction|BindTriggersBeginOverlap (Variables|BackStage|GetBackAnswerTriggers))
  (CallFunction|BindTriggersBeginOverlap (Variables|FrontStage|GetFrontAnswerTriggers)))

(event Custom|HandleLoadedStage
  (params (Level :type Level%20Streaming%20Dynamic%20Object%20Reference))
  ;[1 1 1] Load Stage
  (bind _returnvalue (CallFunction|GetFlagMaster))
  (Class|OsgsBPIFlagMasterStage|SetStandbyStage(Message) _returnvalue Level))

(event Custom|ToggleLoadStage
  (params (Back :type Boolean))
  ;[1 1 1] Load Stage
  (if Back
    (Utilities|FlowControl|DoOnce false :!label _label
      (:Completed
        (Utilities|FlowControl|Sequence
          (:then_0
            _)
          (:then_1
            (goto _label_2 Reset)))))
    (else
      (Utilities|FlowControl|DoOnce false :!label _label_2
        (:Completed
          (Utilities|FlowControl|Sequence
            (:then_0
              _)
            (:then_1
              (goto _label Reset)))))))
  (bind (_success _location _rotation) (CallFunction|GetStageLocationandRotatiion Back))
  (if _success
    (CallFunction|LoadStage (CallFunction|GetStageLevel) _location _rotation)))

(event Custom|SetAnswer
  (params (Back :type Boolean))
  ;[1 1 1] Answer
  (Utilities|FlowControl|DoOnce false
    (:Completed
      (bind _returnvalue (CallFunction|GetFlagMaster))
      (if (Default|ValidAnswer _returnvalue)
        (Default|PostAnswer _returnvalue Back)
        (elif (not (Default|IsEnded _returnvalue))
          (Default|Next _returnvalue))))))

(event Custom|TeleportPlayerToUncheckedAnomalyGuide
  ;[1 1 1] 見つけていないFlagの案内前にテレポート
  (bind _returnvalue (Class|OsgsBPIGameMode|GetStandbyTeleportPlayertoNotFoundsGuide(Message) (Game|GetGameMode)))
  (if (Math|Boolean|ANDBoolean _returnvalue (Utilities|IsValid (Variables|Default|GetNotFoundsGuidePlayerTransform)) (Utilities|IsValid (Game|GetPlayerCharacter 0)))
    (Utilities|FlowControl|DelayUntilNextTick)
    (CallFunction|HandleTeleportPlayertoUncheckedAnomalyGuide)))

(event Custom|BindTriggersBeginOverlap
  (params (Triggers :type Array%20of%20Trigger%20Base%20Object%20References))
  (bind _boundoverlaptriggers (Variables|Default|GetBoundOverlapTriggers))
  ;[1 1 1] Triggers
  (for _array_element Triggers
    (if (not (Utilities|Array|ContainsItem _boundoverlaptriggers _array_element))
      (Utilities|IsValid _array_element
        (:Is%20Valid
          (Utilities|FlowControl|Sequence
            (:then_0
              (Utilities|Array|AddUnique _boundoverlaptriggers _array_element))
            (:then_1
              (EventDispatchers|AssignOnActorBeginOverlap _array_element (delegate Custom|HandleActorBeginOverlap)))))))))

(event Custom|SetupSalvageTriggers
  ;[1 1 1] Triggers
  ;;[1 1 1] Setup Triggers
  (CallFunction|BindTriggersBeginOverlap (Variables|Default|GetSalvageTriggers)))

(event Custom|SetupStageTriggers
  ;[1 1 1] Triggers
  ;;[1 1 1] Setup Triggers
  (CallFunction|BindTriggersBeginOverlap (Variables|BackStage|GetBackStageTriggers))
  (CallFunction|BindTriggersBeginOverlap (Variables|FrontStage|GetFrontStageTriggers)))

(event Custom|HandleActorBeginOverlap
  (params (OverlappedActor :type Actor%20Object%20Reference) (OtherActor :type Actor%20Object%20Reference))
  ;[1 1 1] Triggers
  (if (== OtherActor (Game|GetPlayerCharacter 0)) ; プレイヤーが通過したかどうか（歩くAIなどは無視）
    (Utilities|SwitchTrigger OverlappedActor
      (:Entry
        (CallFunction|Entry))
      (:BackStage
        (CallFunction|ToggleLoadStage true))
      (:FrontStage
        (CallFunction|ToggleLoadStage false))
      (:BackAnswer
        (CallFunction|SetAnswer (Variables|BackStage|GetBackToFoundAnswer)))
      (:FrontAnswer
        (CallFunction|SetAnswer (Variables|FrontStage|GetFrontToFoundAnswer)))
      (:Salvage
        (CallFunction|Salvage)))))

(event EventBeginPlay
  (Utilities|FlowControl|Sequence
    (:then_0
      (CallFunction|SetupTriggers))
    (:then_1
      (CallFunction|TeleportPlayertoUncheckedAnomalyGuide))))

(event Collision|EventActorBeginOverlap
  (params (OtherActor :type Actor%20Object%20Reference)))

(event EventTick
  (params (DeltaSeconds :type Float%20%28single-precision%29)))

(fn ConstructionScript)

(fn GetStageLocationandRotatiion
  (params (Back :type Boolean))
  (bind _frontstagetransform (Variables|FrontStage|GetFrontStageTransform))
  (bind _backstagetransform (Variables|BackStage|GetBackStageTransform))
  (bind _returnvalue (select Back _backstagetransform _frontstagetransform))
  (bind _returnvalue_2 (Transformation|GetActorTransform _returnvalue))
  (Utilities|IsValid _returnvalue
    (:Is%20Valid
      (return true (.location _returnvalue_2) (.rotation _returnvalue_2)))
    (:Is%20Not%20Valid
      (return false "0, 0, 0" "0, 0, 0"))))

(fn GetStageLevel
  (return (Variables|Default|GetMainStageLevel)))