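; Level helper actor for the Top map, the spawn point after startup, clear, restart, trap death or fall salvage, keeping it free of anomalies.
; On BeginPlay it passes MainLevelInstance to the FlagMaster as the current stage and plays an optional sound.
; It polls every 0.1 seconds until flag actors exist, then once forces each one's flag component to false.
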(event EventBeginPlay
  (bind _audio (Variables|Default|GetAudio))
  (bind _sound (Variables|Default|GetSound))
  (Utilities|FlowControl|Sequence
    (:then_0
      (bind _returnvalue (CallFunction|GetFlagMaster))
      (Class|OsgsBPIFlagMasterStage|SetCurrentStage(Message) _returnvalue (Variables|Default|GetMainLevelInstance)))
    (:then_1
      (Utilities|IsValid _sound
        (:Is%20Valid
          (Utilities|FlowControl|Sequence
            (:then_0
              (Audio|Components|Audio|SetSound _audio _sound))
            (:then_1
              (Audio|Components|Audio|Play _audio 0.0))))))
    (:then_2
      ;[1 1 1] 初期表示マップ（起動時・クリア直後・リスタート直後・トラップ死直後・落下サルベージ直後のスポーン地点）ではフラグを立たせない（異変を発生させない）対応
      (bind _outactors (Actor|GetAllActorsOfClass "/Game/Findloople/FLE_BP_FlagActor.FLE_BP_FlagActor_C" :!label _label))
      (if (Utilities|Array|IsNotEmpty _outactors)
        (Utilities|FlowControl|DoOnce false
          (:Completed
            (for _array_element _outactors
              (bind _returnvalue_2 (Default|GetFlagComponent _array_element))
              (Default|HandleFlagChanged _returnvalue_2 false))))
        (else
          (Utilities|FlowControl|Delay 0.1)
          (goto _label))))))

(event Collision|EventActorBeginOverlap
  (params (OtherActor :type Actor%20Object%20Reference)))

(event EventTick
  (params (DeltaSeconds :type Float%20%28single-precision%29)))

(fn ConstructionScript)