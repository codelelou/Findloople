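; Blueprint function library of static helpers for the Findloople game.
; It supplies game info and credit strings: an MIT license notice, an empty "other" credit, and an Unreal Engine trademark notice formatted with the title and year from GetGameInfo.
; It also fetches the flag master message from the GameInstance and the answer user widget from the GameMode's answer component, if that component exists.
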(fn GetFlagMaster
  (bind _returnvalue (Class|OsgsBPIGameInstance|GetFlagMaster(Message) (Game|GetGameInstance)))
  (return _returnvalue))

(fn GetGameInfo
  (return "Findloople" "**********" "**********" 2024))

(fn GetFindloopleCredit
  (return "Findloople 
MIT License 
Copyright (c) 2024 CodeLelou 
Permission is hereby granted, free of charge, to any person obtaining a copy of this software and associated documentation files (the \"Software\"), to deal in the Software without restriction, including without limitation the rights to use, copy, modify, merge, publish, distribute, sublicense, and/or sell copies of the Software, and to permit persons to whom the Software is furnished to do so, subject to the following conditions: 
The above copyright notice and this permission notice shall be included in all copies or substantial portions of the Software. 
THE SOFTWARE IS PROVIDED \"AS IS\", WITHOUT WARRANTY OF ANY KIND, EXPRESS OR IMPLIED, INCLUDING BUT NOT LIMITED TO THE WARRANTIES OF MERCHANTABILITY, FITNESS FOR A PARTICULAR PURPOSE AND NONINFRINGEMENT. IN NO EVENT SHALL THE AUTHORS OR COPYRIGHT HOLDERS BE LIABLE FOR ANY CLAIM, DAMAGES OR OTHER LIABILITY, WHETHER IN AN ACTION OF CONTRACT, TORT OR OTHERWISE, ARISING FROM, OUT OF OR IN CONNECTION WITH THE SOFTWARE OR THE USE OR OTHER DEALINGS IN THE SOFTWARE."))

(fn GetUnrealEngineCredit
  (bind (_title _version _copyright _year) (CallFunction|GetGameInfo))
  (return (Utilities|Text|FormatText (Utilities|Text|MakeLiteralText "Unreal Engine 
{ProductName} uses Unreal® Engine. Unreal® is a trademark or registered trademark of Epic Games, Inc. in the United States of America and elsewhere. Unreal® Engine, Copyright 1998 – {Year}, Epic Games, Inc. All rights reserved.") _title (Utilities|String|ToString(Integer) _year))))

(fn GetOtherCredit
  (return ""))

(fn GetAnswerUserWidget
  (bind _returnvalue (Game|GetGameMode))
  (bind _returnvalue_2 (Actor|GetComponentbyClass _returnvalue "/Game/Osagashi/Blueprint/Answer/Osgs_BP_Answer_ActorComponent_Base.Osgs_BP_Answer_ActorComponent_Base_C"))
  (Utilities|IsValid _returnvalue_2
    (:Is%20Valid
      (bind _returnvalue_3 (Default|GetUserWidget _returnvalue_2))
      (return _returnvalue_3))
    (:Is%20Not%20Valid
      (return 0))))