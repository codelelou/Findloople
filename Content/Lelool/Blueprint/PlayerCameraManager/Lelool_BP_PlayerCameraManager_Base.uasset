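; Base PlayerCameraManager that provides zoom and left/right lean for the character camera.
; Timelines drive both, reversing at higher play rate on stop, with DoOnce and Gate nodes controlling re-entry.
; Zoom lerps camera FOV toward a narrow angle unless a visible zoom-blocking interface widget exists.
; Both broadcast change dispatchers; UpdateLean is an empty hook for child classes implementing lean through camera transforms.
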(event Custom|UpdateLean
  (params (Left :type Boolean) (Alpha :type Float%20%28double-precision%29))
  ;[1 1 1] Lean
)

(event Custom|StartLeanRight
  ;[1 1 1] Lean
  (Utilities|FlowControl|DoOnce false
    (:Completed
      (Utilities|FlowControl|Gate false
        (:Exit
          (Utilities|FlowControl|Sequence
            (:then_0
              (Utilities|FlowControl|Gate false) ; enters at Close
            )
            (:then_1
              (CallFunction|StartLean false))))))))

(event Custom|StartLean
  (params (Left :type Boolean))
  ;[1 1 1] Lean
  (Utilities|FlowControl|Sequence
    (:then_0
      (Components|Timeline|SetPlayRate (Variables|Default|GetLeanTL) 1.0))
    (:then_1
      (bind (_direction _lean) (Timeline|LeanTL Play)
        (:Update
          (CallFunction|CallLeanChangedEventDispatcher true Left _lean :!label _label))
        (:Finished
          (Utilities|FlowControl|Sequence
            (:then_0
              (switch Utilities|FlowControl|Switch|SwitchonETimelineDirection _direction
                (:Forward
                  (goto _label))
                (:Backward
                  (CallFunction|CallLeanChangedEventDispatcher false Left _lean))))
            (:then_1
              (Utilities|FlowControl|DoOnce false) ; enters at Reset
            )
            (:then_2
              (Utilities|FlowControl|DoOnce false) ; enters at Reset
            )))))))

(event Custom|StopLeaningLeft
  ;[1 1 1] Lean
  (if (stale Custom|StartLean Left)
    (CallFunction|StopLeaning)))

(event Custom|Zoom
  (bind _zoomtl (Variables|Default|GetZoomTL))
  ;[1 1 1] FOV (Zoom)
  (Utilities|FlowControl|DoOnce false
    (:Completed
      (if (CallFunction|CanZoom)
        (Utilities|FlowControl|Sequence
          (:then_0
            (Components|Timeline|SetPlayRate _zoomtl 1.0))
          (:then_1
            (bind (_direction _fov) (Timeline|ZoomTL Play)
              (:Update
                (CallFunction|CallZoomChangedEventDispatcher true _fov _direction :!label _label))
              (:Finished
                (switch Utilities|FlowControl|Switch|SwitchonETimelineDirection _direction
                  (:Forward
                    (goto _label))
                  (:Backward
                    (CallFunction|CallZoomChangedEventDispatcher false _fov _direction))))))
          (:then_2
            (Utilities|FlowControl|DoOnce true) ; enters at Reset
          ))
        (else
          (Utilities|FlowControl|DoOnce true) ; enters at Reset
        )))))

(event Custom|StopLeaningRight
  ;[1 1 1] Lean
  (if (not (stale Custom|StartLean Left))
    (CallFunction|StopLeaning)))

(event Custom|SetFOV
  (params (NewFOV :type Float%20%28double-precision%29))
  (bind _returnvalue (Game|Player|GetOwningPlayerController))
  (bind _returnvalue_2 (Pawn|GetControlledPawn _returnvalue))
  (bind _returnvalue_3 (Actor|GetComponentsByClass _returnvalue_2 "/Script/Engine.CameraComponent"))
  ;[1 1 1] FOV (Zoom)
  (for _array_element _returnvalue_3
    (if (Components|Activation|IsActive _array_element)
      (Camera|SetFieldOfView _returnvalue_3 NewFOV))))

(event Custom|SetBeforeCameraFOVAngle
  (params (FOV :type Float%20%28double-precision%29))
  ;[1 1 1] FOV (Zoom)
)

(event Custom|StopZooming
  (bind _zoomtl (Variables|Default|GetZoomTL))
  ;[1 1 1] FOV (Zoom)
  (Utilities|FlowControl|DoOnce true
    (:Completed
      (Utilities|FlowControl|Sequence
        (:then_0
          (bind (_direction _fov) (Timeline|ZoomTL Stop)
            (:Update
              (CallFunction|CallZoomChangedEventDispatcher true _fov _direction :!label _label))
            (:Finished
              (switch Utilities|FlowControl|Switch|SwitchonETimelineDirection _direction
                (:Forward
                  (goto _label))
                (:Backward
                  (CallFunction|CallZoomChangedEventDispatcher false _fov _direction))))))
        (:then_1
          (Components|Timeline|SetPlayRate _zoomtl 1e+01))
        (:then_2
          (Timeline|ZoomTL Reverse))
        (:then_3
          (Utilities|FlowControl|DoOnce false) ; enters at Reset
        )))))

(event Custom|CallLeanChangedEventDispatcher
  (params (Leaning :type Boolean) (Left :type Boolean) (Alpha :type Float%20%28double-precision%29))
  ;[1 1 1] Lean
  (bind _output_get (Variables|Default|SetLeaning Leaning))
  (Utilities|FlowControl|Sequence
    (:then_0
      (if _output_get
        (CallFunction|UpdateLean Left Alpha)))
    (:then_1
      (Default|CallOnLeanChanged _output_get Left Alpha))))

(event Custom|StopLeaning
  ;[1 1 1] Lean
  (Utilities|FlowControl|Sequence
    (:then_0
      (bind (_direction _lean) (Timeline|LeanTL Stop)
        (:Update
          (CallFunction|CallLeanChangedEventDispatcher true (stale Custom|StartLean Left) _lean :!label _label))
        (:Finished
          (Utilities|FlowControl|Sequence
            (:then_0
              (switch Utilities|FlowControl|Switch|SwitchonETimelineDirection _direction
                (:Forward
                  (goto _label))
                (:Backward
                  (CallFunction|CallLeanChangedEventDispatcher false (stale Custom|StartLean Left) _lean))))
            (:then_1
              (Utilities|FlowControl|DoOnce false) ; enters at Reset
            )
            (:then_2
              (Utilities|FlowControl|DoOnce false) ; enters at Reset
            )))))
    (:then_1
      (Components|Timeline|SetPlayRate (Variables|Default|GetLeanTL) 1e+01))
    (:then_2
      (Timeline|LeanTL Reverse))
    (:then_3
      (Utilities|FlowControl|Gate false) ; enters at Open
    )
    (:then_4
      (Utilities|FlowControl|Gate false) ; enters at Open
    )))

(event Custom|CallZoomChangedEventDispatcher
  (params (Zooming :type Boolean) (Alpha :type Float%20%28double-precision%29) (Direction :type ETimelineDirection%20Enum :default "Forward"))
  ;[1 1 1] FOV (Zoom)
  (bind _output_get (Variables|Default|SetZooming Zooming))
  (Utilities|FlowControl|Sequence
    (:then_0
      (Utilities|FlowControl|DoOnce false :!label _label
        (:Completed
          (CallFunction|SetBeforeCameraFOVAngle (Camera|GetFOVAngle (Game|GetPlayerCameraManager 0))))))
    (:then_1
      (if (not _output_get)
        (goto _label Reset)))
    (:then_2
      (CallFunction|SetFOV (Math|Float|Lerp (stale Custom|SetBeforeCameraFOVAngle FOV) 45.0 Alpha)))
    (:then_3
      (Default|CallOnZoomChanged _output_get Alpha Direction))))

(event Custom|StartLeanLeft
  ;[1 1 1] Lean
  (Utilities|FlowControl|DoOnce false
    (:Completed
      (Utilities|FlowControl|Gate false
        (:Exit
          (Utilities|FlowControl|Sequence
            (:then_0
              (Utilities|FlowControl|Gate false) ; enters at Close
            )
            (:then_1
              (CallFunction|StartLean true))))))))

(event EventBeginPlay)

(event Collision|EventActorBeginOverlap
  (params (OtherActor :type Actor%20Object%20Reference)))

(event EventTick
  (params (DeltaSeconds :type Float%20%28single-precision%29)))

(event EventZoomatCharacterCamera
  (CallFunction|Zoom))

(event EventStopZoomingatCharacterCamera
  (CallFunction|StopZooming))

(event EventLeanLeftatCharacterCamera
  (CallFunction|StartLeanLeft))

(event EventStopLeaningLeftatCharacterCamera
  (CallFunction|StopLeaningLeft))

(event EventLeanRightatCharacterCamera
  (CallFunction|StartLeanRight))

(event EventStopLeaningRightatCharacterCamera
  (CallFunction|StopLeaningRight))

(event EventStopLeaningatCharacterCamera
  (CallFunction|StopLeaning))

(fn ConstructionScript)

(fn CanZoom
  (bind _foundwidgets (Class|WidgetBlueprintLibrary|GetAllWidgetswithInterface (Variables|Zoom|GetZoomBlockWidgetInterfaceClass) true))
  (for _array_element _foundwidgets
    (if (Widget|IsVisible _array_element)
      (return false)))
  (return true))

(fn GetBlockZoomWidgets
  (return 0))

(fn GetZoomingMaxWalkSpeed
  (return 0.0))

(fn LeaningatCharacterCamera
  (return (Variables|Default|GetLeaning)))

(fn ZoomingatCharacterCamera
  (return (Variables|Default|GetZooming)))