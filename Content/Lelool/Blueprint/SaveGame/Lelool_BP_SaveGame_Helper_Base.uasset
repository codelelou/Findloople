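; Base helper object that manages one save game slot and its SaveGame instance, using its outer object as world context.
; Load runs once, creates a fresh object from SaveGameClass if none is found, and always reports success.
; Save writes synchronously behind a re-entry guard, Reset saves a fresh object, and Delete recreates it after clearing the slot.
; Event dispatchers announce load, save, delete and object changes.
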(event Custom|Load
  (Utilities|FlowControl|DoOnce false
    (:Completed
      (bind _returnvalue (CallFunction|GetSlotName))
      (Utilities|FlowControl|Sequence
        (:then_0
          (Default|CallOnLoadStart))
        (:then_1
          (bind _returnvalue_2 (SaveGame|LoadGamefromSlot _returnvalue))
          (Utilities|FlowControl|Sequence
            (:then_0
              (Utilities|IsValid _returnvalue_2
                (:Is%20Valid
                  (CallFunction|SetSaveGame _returnvalue_2))
                (:Is%20Not%20Valid
                  (CallFunction|Factory))))
            (:then_1
              (Variables|Default|SetLoadCompleted true))
            (:then_2
              (CallFunction|CallLoadCompletedEventDispatcher _returnvalue_2 true))))))))

(event Custom|SetSaveGame
  (params (SaveGame :type Save%20Game%20Object%20Reference))
  (if (!= SaveGame (stale _output_get))
    (Default|CallOnSaveGameChanged SaveGame (stale _output_get))
    (bind _output_get (Variables|Default|SetSaveGame SaveGame))))

(event Custom|Save
  (Utilities|FlowControl|DoOnce false :!label _label
    (:Completed
      (Utilities|FlowControl|Sequence
        (:then_0
          (bind _returnvalue (CallFunction|GetSaveGame))
          (Default|CallOnSaveStartSaveGame _returnvalue))
        (:then_1
          (bind _returnvalue_2 (CallFunction|GetSaveGame))
          (bind _returnvalue_3 (CallFunction|GetSlotName))
          (bind _returnvalue_4 (SaveGame|SaveGametoSlot _returnvalue_2 _returnvalue_3))
          (Utilities|FlowControl|Sequence
            (:then_0
              (CallFunction|CallSaveCompletedEventDispatcher _returnvalue_2 _returnvalue_4))
            (:then_1
              (goto _label Reset))))))))

(event Custom|Reset
  (bind _returnvalue (CallFunction|FactoryResetSaveGame))
  (Utilities|FlowControl|Sequence
    (:then_0
      (CallFunction|SetSaveGame _returnvalue))
    (:then_1
      (CallFunction|Save))))

(event Custom|Factory
  (bind _returnvalue (CallFunction|CreateSaveGameObject))
  (CallFunction|SetSaveGame _returnvalue))

(event Custom|CallSaveCompletedEventDispatcher
  (params (SaveGame :type Save%20Game%20Object%20Reference) (Success :type Boolean))
  (Default|CallOnSaveCompletedSaveGame SaveGame Success))

(event Custom|CallLoadCompletedEventDispatcher
  (params (SaveGame :type Save%20Game%20Object%20Reference) (Success :type Boolean))
  (Default|CallOnLoadCompleted SaveGame Success))

(event EventSaveSaveGame
  (CallFunction|Save))

(fn GetWorldContextObject
  (return (Utilities|GetOuterObject self)))

(fn CreateSaveGameObject
  (bind _returnvalue (SaveGame|CreateSaveGameObject (Variables|Default|GetSaveGameClass)))
  (return _returnvalue))

(fn GetSlotName
  (return (Variables|Default|GetSlotName)))

(fn Delete
  (bind _returnvalue (CallFunction|GetSlotName))
  (bind _returnvalue_2 (SaveGame|DeleteGameinSlot _returnvalue))
  (Utilities|FlowControl|Sequence
    (:then_0
      (if _returnvalue_2
        (CallFunction|Factory)))
    (:then_1
      (Default|CallOnDeleted _returnvalue_2))
    (:then_2
      (return _returnvalue_2))))

(fn FactoryResetSaveGame
  (bind _returnvalue (CallFunction|CreateSaveGameObject))
  (return _returnvalue))

(fn IsLoadCompleted
  (return (Variables|Default|GetLoadCompleted)))

(fn GetSaveGame
  (return (Variables|Default|GetSaveGame)))

(fn IsSaveGameLoadCompleted
  (bind _returnvalue (CallFunction|IsLoadCompleted))
  (return _returnvalue))