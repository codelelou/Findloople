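; Base GameInstance for Osagashi Advance that loads the settings, achievement and gameplay save games on Init.
; Each save game has a lazily constructed helper object, exposed through getters.
; Load callbacks check all three helpers and fire OnLoadSaveGamesCompleted once when all are done.
; Loaded settings also drive BGM, sound effect and voice volumes through sound mix class overrides, applied a tick later.
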(event Custom|HandleGameplayLoadCompleted
  (params (SaveGame :type Save%20Game%20Object%20Reference) (Success :type Boolean))
  ;[1 1 1] Gameplay (Main Game)
  (CallFunction|HandleLoadSaveGameCompleted (stale Custom|SetupGameplay _returnvalue)))

(event Custom|HandleGameplaySaveGameChanged
  (params (SaveGame :type Save%20Game%20Object%20Reference) (BeforeSaveGame :type Save%20Game%20Object%20Reference))
  ;[1 1 1] Gameplay (Main Game)
)

(event Custom|SetSoundMixClassOverride
  (params (InSoundClass :type Sound%20Class%20Object%20Reference) (Volume :type Float%20%28single-precision%29))
  ;[1 1 1] Sound
  (Utilities|IsValid InSoundClass
    (:Is%20Valid
      (Audio|SetSoundMixClassOverride (Variables|Settings|GetSoundMix) InSoundClass Volume 1.0 1.0 true))))

(event Custom|SetupGameplay
  ;[1 1 1] Gameplay (Main Game)
  (bind _returnvalue (Gameplay|GetGameplaySaveGameHelper))
  (Utilities|IsValid _returnvalue
    (:Is%20Valid
      (Utilities|FlowControl|Sequence
        (:then_0
          (EventDispatchers|AssignOnLoadCompleted _returnvalue (delegate Custom|HandleGameplayLoadCompleted)))
        (:then_1
          (EventDispatchers|AssignOnSaveGameChanged _returnvalue (delegate Custom|HandleGameplaySaveGameChanged)))
        (:then_2
          (Default|Load _returnvalue))))))

(event Custom|LoadSaveGames
  ;[1 1 1] SaveGame
  (Utilities|FlowControl|DoOnce false
    (:Completed
      (Utilities|FlowControl|Sequence
        (:then_0
          (CallFunction|SetupSettings))
        (:then_1
          (CallFunction|SetupAchievement))
        (:then_2
          (CallFunction|SetupGameplay))))))

(event Custom|HandleLoadSaveGameCompleted
  (params (Helper :type Lelool%20BP%20Save%20Game%20Helper%20Base%20Object%20Reference))
  ;[1 1 1] SaveGame
  (bind _returnvalue (CallFunction|IsLoadSaveGamesCompleted))
  (if _returnvalue
    (Utilities|FlowControl|DoOnce false
      (:Completed
        (CallFunction|HandleLoadSaveGamesCompleted)))))

(event Custom|SetupSettings
  ;[1 1 1] SettingsSaveGame
  (bind _returnvalue (Settings|GetSettingsSaveGameHelper))
  (Utilities|IsValid _returnvalue
    (:Is%20Valid
      (Utilities|FlowControl|Sequence
        (:then_0
          (EventDispatchers|AssignOnLoadCompleted _returnvalue (delegate Custom|HandleSettingsLoadCompleted)))
        (:then_1
          (EventDispatchers|AssignOnSaveGameChanged _returnvalue (delegate Custom|HandleSettingsSaveGameChanged)))
        (:then_2
          (Default|Load _returnvalue))))))

(event Custom|HandleSettingsLoadCompleted
  (params (SaveGame :type Save%20Game%20Object%20Reference) (Success :type Boolean))
  ;[1 1 1] SettingsSaveGame
  (Utilities|FlowControl|Sequence
    (:then_0
      (CallFunction|UpdateSoundClasses))
    (:then_1
      (CallFunction|HandleLoadSaveGameCompleted (stale Custom|SetupSettings _returnvalue)))))

(event Custom|HandleSettingsSaveGameChanged
  (params (SaveGame :type Save%20Game%20Object%20Reference) (BeforeSaveGame :type Save%20Game%20Object%20Reference))
  ;[1 1 1] SettingsSaveGame
)

(event Custom|HandleLoadSaveGamesCompleted
  ;[1 1 1] SaveGame
  (Utilities|FlowControl|DoOnce false
    (:Completed
      (Default|CallOnLoadSaveGamesCompleted))))

(event Custom|HandleLoadAchievementCompleted
  (params (SaveGame :type Save%20Game%20Object%20Reference) (Success :type Boolean))
  ;[1 1 1] Achievement
  (CallFunction|HandleLoadSaveGameCompleted (stale Custom|SetupAchievement _returnvalue)))

(event Custom|SetupAchievement
  ;[1 1 1] Achievement
  (bind _returnvalue (Achievement|GetAchievementSaveGameHelper))
  (Utilities|FlowControl|Sequence
    (:then_0
      (EventDispatchers|AssignOnLoadCompleted _returnvalue (delegate Custom|HandleLoadAchievementCompleted)))
    (:then_1
      (Default|Load _returnvalue))))

(event EventInit
  (|CallParentFunction)
  (CallFunction|LoadSaveGames))

(event EventSaveSettingsSaveGame
  ;[1 1 1] SettingsSaveGame
  (bind _returnvalue (Settings|GetSettingsSaveGameHelper))
  (Class|LeloolBPISaveGameHelper|SaveSaveGame(Message) _returnvalue))

(event EventResetSettingsSaveGame
  ;[1 1 1] SettingsSaveGame
  (bind _returnvalue (Settings|GetSettingsSaveGameHelper))
  (Default|Reset _returnvalue))

(event EventUpdateSoundClasses
  (bind _soundmix (Variables|Settings|GetSoundMix))
  ;[1 1 1] Sound
  (Utilities|IsValid _soundmix
    (:Is%20Valid
      (Utilities|FlowControl|DelayUntilNextTick)
      (bind _returnvalue (Settings|GetSettings))
      (Utilities|FlowControl|Sequence
        (:then_0
          (Utilities|FlowControl|Sequence
            (:then_0
              (bind _returnvalue_2 (Class|LeloolBPISaveGameSettings|GetBGMSettingsinSaveGame(Message) _returnvalue))
              (CallFunction|SetSoundMixClassOverride "/Game/Osagashi/Sound/Osgs_SoundClass_BGM.Osgs_SoundClass_BGM" _returnvalue_2))
            (:then_1
              (bind _returnvalue_3 (Class|LeloolBPISaveGameSettings|GetSoundEffectSettingsinSaveGame(Message) _returnvalue))
              (CallFunction|SetSoundMixClassOverride "/Game/Osagashi/Sound/Osgs_SoundClass_SoundEffect.Osgs_SoundClass_SoundEffect" _returnvalue_3))
            (:then_2
              (bind _returnvalue_4 (Class|LeloolBPISaveGameSettings|GetVoiceSettingsinSaveGame(Message) _returnvalue))
              (CallFunction|SetSoundMixClassOverride "/Game/Osagashi/Sound/Osgs_SoundClass_Voice.Osgs_SoundClass_Voice" _returnvalue_4))))
        (:then_1
          (Audio|PushSoundMixModifier _soundmix))))))

(fn GetSettings
  (bind _returnvalue (Settings|GetSettingsSaveGameHelper))
  (bind _returnvalue_2 (Class|LeloolBPISaveGameHelper|GetSaveGame(Message) _returnvalue))
  (return _returnvalue_2))

(fn GetSettingsSaveGameHelper
  (Utilities|IsValid (stale _output_get)
    (:Is%20Valid
      _)
    (:Is%20Not%20Valid
      (bind _returnvalue (Game|ConstructObjectfromClass "/Game/Osagashi_Advance/Blueprint/SaveGame/Settings/Osgs_Advance_BP_SaveGame_Helper_Settings.Osgs_Advance_BP_SaveGame_Helper_Settings_C"))
      (bind _output_get (Variables|Settings|SetSettingsSaveGameHelper _returnvalue))))
  (return _output_get))

(fn GetAchievementSaveGameHelper
  (Utilities|IsValid (stale _output_get)
    (:Is%20Valid
      _)
    (:Is%20Not%20Valid
      (bind _returnvalue (Game|ConstructObjectfromClass "/Game/Osagashi_Advance/Blueprint/SaveGame/Achievement/Osgs_Advance_BP_SaveGame_Helper_Achievement.Osgs_Advance_BP_SaveGame_Helper_Achievement_C"))
      (bind _output_get (Variables|Achievement|SetAchievementSaveGameHelper _returnvalue))))
  (return _output_get))

(fn GetGameplaySaveGameHelper
  (Utilities|IsValid (stale _output_get)
    (:Is%20Valid
      _)
    (:Is%20Not%20Valid
      (bind _returnvalue (Game|ConstructObjectfromClass "/Game/Osagashi_Advance/Blueprint/SaveGame/Gameplay/Osgs_Advance_BP_SaveGame_Helper_Gameplay.Osgs_Advance_BP_SaveGame_Helper_Gameplay_C"))
      (bind _output_get (Variables|Gameplay|SetGameplaySaveGameHelper _returnvalue))))
  (return _output_get))

(fn GetAchievementHelper
  (bind _returnvalue (Achievement|GetAchievementSaveGameHelper))
  (return _returnvalue))

(fn GetGameplayHelper
  (bind _returnvalue (Gameplay|GetGameplaySaveGameHelper))
  (return _returnvalue))

(fn GetSettingsHelper
  (bind _returnvalue (Settings|GetSettingsSaveGameHelper))
  (return _returnvalue))

(fn GetSettingsSaveGame
  (bind _returnvalue (Settings|GetSettings))
  (return _returnvalue))

(fn IsLoadSaveGamesCompleted
  (Utilities|FlowControl|Sequence
    (:then_0
      (bind _returnvalue (Settings|GetSettingsSaveGameHelper)))
    (:then_1
      (bind _returnvalue_2 (Gameplay|GetGameplaySaveGameHelper)))
    (:then_2
      (bind _returnvalue_3 (Achievement|GetAchievementSaveGameHelper)))
    (:then_3
      (for _array_element (Utilities|Array|MakeArray _returnvalue _returnvalue_2 _returnvalue_3)
        (bind _returnvalue_4 (Default|IsLoadCompleted _array_element))
        (if (not _returnvalue_4)
          (return false)))
      (return true))))