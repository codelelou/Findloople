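; Game instance for Osagashi Advance that applies loaded save data to the flag master and the player camera.
; After the gameplay load handler runs, it passes the gameplay save helper to FlagMaster to restore flags.
; Settings load and change handlers read the FOV through a message call on the save game and set it as player 0's camera manager DefaultFOV.
; Each override calls its parent handler first.
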(event Custom|UpdateFOVBySaveGame
  (params (SaveGame :type Object%20Object%20Reference))
  ;[1 1 1] FOV
  (bind _returnvalue (Class|LeloolBPISaveGameSettings|GetFOVSettingsinSaveGame(Message) SaveGame))
  (Variables|/Script/Engine.PlayerCameraManager|SetDefaultFOV (Game|GetPlayerCameraManager 0) _returnvalue))

(event EventHandleGameplayLoadCompleted
  (params (SaveGame :type Save%20Game%20Object%20Reference) (Success :type Boolean))
  (|CallParentFunction SaveGame Success)
  ;[1 1 1] セーブデータ読込後にFlagMasterをリストア
  (bind _returnvalue (CallFunction|GetFlagMaster))
  (bind _returnvalue_2 (CallFunction|GetGameplayHelper))
  (Class|OsgsAdvanceBPIFlagMasterSaveGame|SetSaveGameHelper(Message) _returnvalue _returnvalue_2))

(event EventHandleSettingsLoadCompleted
  (params (SaveGame :type Save%20Game%20Object%20Reference) (Success :type Boolean))
  ;[1 1 1] FOV
  (|CallParentFunction SaveGame Success)
  (CallFunction|UpdateFOVbySaveGame SaveGame))

(event EventHandleSettingsSaveGameChanged
  (params (SaveGame :type Save%20Game%20Object%20Reference) (BeforeSaveGame :type Save%20Game%20Object%20Reference))
  ;[1 1 1] FOV
  (|CallParentFunction SaveGame BeforeSaveGame)
  (CallFunction|UpdateFOVbySaveGame SaveGame))