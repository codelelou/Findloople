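; Gameplay HUD Blueprint for Osagashi Advance that shows the aiming reticle and the pause menu.
; BeginPlay adds the reticle widget to the viewport once.
; Show and hide pause events forward a paused flag to a lazily created, cached pause widget, which handles its own visibility and pause permission.
; That same pause widget also supplies the main CommonUI activatable widget container.
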(event Custom|ShowPause
  ;[1 1 1] GamePaused（表示非表示・一時停止許可の制御はWidgetで実装）
  (CallFunction|SetGamePaused true))

(event Custom|HidePause
  ;[1 1 1] GamePaused（表示非表示・一時停止許可の制御はWidgetで実装）
  (CallFunction|SetGamePaused false))

(event Custom|ShowReticle
  ;[1 1 1] Reticle（表示非表示の制御はWidgetで実装）
  (Utilities|FlowControl|DoOnce false
    (:Completed
      (bind _returnvalue (UserInterface|CreateWidget (Variables|Reticle|GetReticleUserWidget%20Class)))
      (UserInterface|Viewport|AddtoViewport _returnvalue (Variables|Reticle|GetReticleWidgetZOrder)))))

(event Custom|SetGamePaused
  (params (Paused :type Boolean))
  ;[1 1 1] GamePaused（表示非表示・一時停止許可の制御はWidgetで実装）
  (bind _returnvalue (GamePaused|GetGamePausedWidget))
  (Class|OsgsAdvanceBPIPause|SetGamePaused(Message) _returnvalue Paused))

(event EventBeginPlay
  (|CallParentFunction)
  (CallFunction|ShowReticle))

(event Collision|EventActorBeginOverlap
  (params (OtherActor :type Actor%20Object%20Reference))
  (|CallParentFunction OtherActor) ; このノードは無効になっているため呼び出せません。\n機能をビルドするにはピンをドラッグしてください。
)

(event EventTick
  (params (DeltaSeconds :type Float%20%28single-precision%29))
  (|CallParentFunction DeltaSeconds) ; このノードは無効になっているため呼び出せません。\n機能をビルドするにはピンをドラッグしてください。
)

(event EventShowPauseMenu
  (CallFunction|ShowPause))

(event EventHidePauseMenu
  (CallFunction|HidePause))

(fn ConstructionScript
  (|CallParentFunction))

(fn GetMainUserWidgetContainer
  (bind _returnvalue (CallFunction|GetPause))
  (bind _returnvalue_2 (Class|OsgsAdvanceBPIMainUserWidget|GetCommonActivatableWidgetContainer(Message) _returnvalue))
  (return _returnvalue_2))

(fn GetPause
  (bind _returnvalue (GamePaused|GetGamePausedWidget))
  (return _returnvalue))

(fn GetGamePausedWidget
  (Utilities|IsValid (stale _output_get)
    (:Is%20Valid
      (return (stale _output_get)))
    (:Is%20Not%20Valid
      (bind _returnvalue (UserInterface|CreateWidget (Variables|GamePaused|GetPauseUserWidgetClass)))
      (Utilities|FlowControl|Sequence
        (:then_0
          (bind _output_get (Variables|GamePaused|SetPauseUserWidget _returnvalue)))
        (:then_1
          (UserInterface|Viewport|AddtoViewport _returnvalue (Variables|GamePaused|GetPauseWidgetZOrder)))
        (:then_2
          (return _output_get))))))