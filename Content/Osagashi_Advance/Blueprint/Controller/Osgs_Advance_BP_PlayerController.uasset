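; Player controller for Osagashi Advance that sets up game-only input and applies the saved field-of-view setting.
; On BeginPlay it hides the cursor, gets the settings helper from the Game Instance and applies its current save game.
; It also binds to the helper's save-completed event, so each save reapplies the FOV as the camera manager's DefaultFOV, without checking the success flag.
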(event Custom|HandleSettingsSaveGameChanged
  (params (SaveGame :type Save%20Game%20Object%20Reference))
  (bind _returnvalue (Class|LeloolBPISaveGameSettings|GetFOVSettingsinSaveGame(Message) SaveGame))
  (Variables|/Script/Engine.PlayerCameraManager|SetDefaultFOV (Game|GetPlayerCameraManager 0) _returnvalue))

(event Custom|HandleSaveCompletedSettingsSaveGame
  (params (SaveGame :type Save%20Game%20Object%20Reference) (Success :type Boolean))
  (CallFunction|HandleSettingsSaveGameChanged SaveGame))

(event EventBeginPlay
  (|CallParentFunction)
  (Utilities|FlowControl|Sequence
    (:then_0
      (Variables|Default|SetbShowMouseCursor false)
      (Input|SetInputModeGameOnly self false))
    (:then_1
      (bind _returnvalue (Class|LeloolBPIGameInstanceSaveGame|GetSettingsHelper(Message) (Game|GetGameInstance)))
      (Utilities|FlowControl|Sequence
        (:then_0
          (bind _returnvalue_2 (Class|LeloolBPISaveGameHelper|GetSaveGame(Message) _returnvalue))
          (CallFunction|HandleSettingsSaveGameChanged _returnvalue_2))
        (:then_1
          (EventDispatchers|AssignOnSaveCompletedSaveGame _returnvalue (delegate Custom|HandleSaveCompletedSettingsSaveGame)))))))

(event EventTick
  (params (DeltaSeconds :type Float%20%28single-precision%29))
  (|CallParentFunction DeltaSeconds) ; このノードは無効になっているため呼び出せません。\n機能をビルドするにはピンをドラッグしてください。
)

(fn ConstructionScript
  (|CallParentFunction))