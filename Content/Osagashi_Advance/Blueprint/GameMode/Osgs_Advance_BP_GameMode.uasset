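; Game mode Blueprint for the Osagashi Advance game that sets up graphics settings when play begins.
; On BeginPlay it calls SetupGraphicSetting, which checks that a configured graphics settings component class is valid.
; It then spawns a Lelool graphic setting component actor at the world origin, passing that class to it.
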(event Custom|SetupGraphicSetting
  (bind _graphicsettingcomponetclassclass (Variables|Default|GetGraphicSettingComponetClassClass))
  (if (Utilities|IsValidClass _graphicsettingcomponetclassclass)
    (Game|SpawnActorfromClass "/Game/Lelool/Component/GraphicSetting/Lelool_BP_GraphicSettingComponent_Actor.Lelool_BP_GraphicSettingComponent_Actor_C" (Math|Transform|MakeTransform "0, 0, 0") "Undefined" "MultiplyWithRoot" 0 _graphicsettingcomponetclassclass 0)))

(event EventBeginPlay
  (|CallParentFunction)
  (CallFunction|SetupGraphicSetting))

(event EventTick
  (params (DeltaSeconds :type Float%20%28single-precision%29))
  (|CallParentFunction DeltaSeconds) ; このノードは無効になっているため呼び出せません。\n機能をビルドするにはピンをドラッグしてください。
)

(fn ConstructionScript
  (|CallParentFunction))